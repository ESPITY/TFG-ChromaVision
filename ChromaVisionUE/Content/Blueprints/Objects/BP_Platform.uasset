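; BP_Platform is a platform actor that moves vertically from its placed position.
; On BeginPlay it stores its start location and plays the VerticalMovement timeline.
; Each timeline update sets the actor's Z to the start height plus the scaled VerticalOffset track, keeping X and Y fixed.
; Event tracks on the same timeline trigger the AudioUp and AudioDown sounds, keeping audio in step with the motion.
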(event EventBeginPlay
  ;[0.15 0.15 0.15 0.5] Movimiento vertical de la plataforma
  (Variables|Default|SetStartLocation (Transformation|GetActorLocation))
  (bind _verticaloffset (Timeline|VerticalMovement Play)
    (:Update
      (Transformation|SetActorLocation (Math|Vector|MakeVector (.x (Variables|Default|GetStartLocation)) (.y (Variables|Default|GetStartLocation)) (+ (.z (Variables|Default|GetStartLocation)) (* _verticaloffset 1.8e+02))) false false))
    (:SoundUp
      (Audio|Components|Audio|Play (Variables|Default|GetAudioUp) 0.0))
    (:SoundDown
      (Audio|Components|Audio|Play (Variables|Default|GetAudioDown) 0.0))))

(fn ConstructionScript)