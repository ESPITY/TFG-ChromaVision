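; Game mode that switches between a top-down construction mode, with its widget UI, and a play mode.
; ChangeMode stops UDP reception and possesses the first piece-spawned character, or the scene default, then restores its position on return.
; Tag-mapped cameras blend on switching, and a spectator pawn spawned once starts from the current view.
; A DoOnce-guarded timeline rotates the top-down camera in 90-degree steps.
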(event Custom|GetCameras
  ;[0.1274 0.2159 0.5149 0.502] Obtener las referencias de las cámaras (value) y guardarlas en un map con el tag (key)
  (bind _outactors (Actor|GetAllActorsOfClass "/Script/Engine.CameraActor"))
  (for _array_element _outactors
    (Utilities|Map|Add (Variables|Default|GetCameras) (Utilities|Array|Get(acopy) (Variables|/Script/Engine.Actor|GetTags _array_element)) _array_element)))

(event Custom|PossessCharacter
  (params (InPawn :type Pawn%20Object%20Reference))
  (bind _returnvalue (Game|GetPlayerController 0))
  ;[1 0.3059 0.09615 0.5] Poseer al personaje que se recibe como input del Custom Event durante el cambio al modo juego
  (Pawn|Possess (Game|GetPlayerController 0) InPawn)
  (Widget|SetVisibility (Variables|Default|GetConstructionWidget) "Hidden")
  (Input|SetInputModeGameOnly _returnvalue false)
  (Variables|/Script/Engine.PlayerController|SetbShowMouseCursor _returnvalue false))

(event Custom|ToggleCMUI
  (bind _returnvalue (Game|GetPlayerController 0))
  (bind _constructionwidget (Variables|Default|GetConstructionWidget))
  (bind _spectatorcamerawidget (Variables|Default|GetSpectatorCameraWidget))
  ;[0.1651 0.5029 0.1248 0.502] Mostrar/ocultar la interfaz del modo de construcción y la de la SpectatorCamera
  (if (Widget|IsVisible _constructionwidget)
    (Widget|SetVisibility _constructionwidget "Hidden")
    (Input|SetInputModeGameOnly _returnvalue false)
    (Variables|/Script/Engine.PlayerController|SetbShowMouseCursor _returnvalue false)
    (Utilities|IsValid _spectatorcamerawidget
      (:Is%20Valid
        (Widget|SetVisibility _spectatorcamerawidget "Visible")))
    (else
      (Widget|SetVisibility _constructionwidget "Visible")
      (Input|SetInputModeGameandUI _returnvalue 0 "DoNotLock" true false)
      (Variables|/Script/Engine.PlayerController|SetbShowMouseCursor _returnvalue true)
      (Utilities|IsValid _spectatorcamerawidget
        (:Is%20Valid
          (Widget|SetVisibility _spectatorcamerawidget "Hidden"))))))

(event Custom|SwitchCamera
  (params (Camera :type Name))
  (bind _returnvalue (Game|GetPlayerController 0))
  (bind _cameras (Variables|Default|GetCameras))
  (bind _constructionwidget (Variables|Default|GetConstructionWidget))
  (bind (_value _returnvalue_2) (Utilities|Map|Find _cameras Camera))
  ;[0.1274 0.2159 0.5149 0.502] Cambiar de cámara con el tag desde el WBP_ConstructionMode, si estaba la SpectatorCamera activa se desposee y se reactiva su botón
  (if _returnvalue_2
    (Utilities|FlowControl|Sequence
      (:then_0
        (if (Variables|Default|GetbActiveSpectatorCamera)
          (Pawn|UnPossess _returnvalue)
          (Default|EnableBTSpectatorCamera (Variables|Default|GetConstructionWidget))
          (Variables|Default|SetbActiveSpectatorCamera false)))
      (:then_1
        (Utilities|FlowControl|DelayUntilNextTick)
        (Game|Player|SetViewTargetwithBlend _returnvalue _value 0.5 "VTBlend_Cubic" 0.0 false)
        (bind _output_get (Variables|Default|SetCurrentCamera Camera))
        (if (== _output_get "CTopdown")
          (Default|EnableBTCTopdownRot _constructionwidget)
          (else
            (Default|DisableBTCTopdownRot _constructionwidget)))))))

(event Custom|RotateCTopdownRight
  (bind _cameras (Variables|Default|GetCameras))
  (bind (_value _returnvalue) (Utilities|Map|Find _cameras "CTopdown"))
  ;[0.1274 0.2159 0.5149 0.502] Rotar suavemente la cámara cenital 90º a izq./der.
  (Variables|Default|SetRotation -9e+01)
  (if (== (Variables|Default|GetCurrentCamera) "CTopdown")
    (Utilities|FlowControl|DoOnce false
      (:Completed
        (if _returnvalue
          (Variables|Default|SetStartCTopdownRotation (Transformation|GetActorRotation _value))
          (bind _rotationoffset (Timeline|CameraRotation PlayFromStart)
            (:Update
              (Transformation|SetActorRotation _value (Math|Rotator|Lerp(Rotator) (Variables|Default|GetStartCTopdownRotation) (Math|Rotator|MakeRotator (+ (.roll (Variables|Default|GetStartCTopdownRotation)) (Variables|Default|GetRotation)) (.pitch (Variables|Default|GetStartCTopdownRotation)) (.yaw (Variables|Default|GetStartCTopdownRotation))) _rotationoffset true)))
            (:Finished
              (CallFunction|FinishedCRotation))))))))

(event Custom|ChangeMode
  (bind _returnvalue (Game|GetPlayerController 0))
  ;[1 0.3059 0.09615 0.5] Cambio entre modo construcción y modo juego. Gestión de la posesión del personaje por defecto o el 1o spawneado por piezas cuando se cambia a modo juego
  (Utilities|FlowControl|FlipFlop
    (:A
      (Class|UDPReceiver|StopUDPReceiver (Variables|Default|GetUDPReceiver))
      (Class|CheckBox|SetIsChecked (Variables|/Game/UI/WBP_ConstructionMode.WBP_ConstructionMode_C|GetCB_UDPConnection (Variables|Default|GetConstructionWidget)) false)
      (bind _outactors (Actor|GetAllActorsOfClasswithTag "/Game/Blueprints/BP_Character.BP_Character_C" "Player"))
      (if (> (Utilities|Array|Length _outactors) 1)
        ;;[0.05926 0 0.3647 0.5] Poseer al 1er personaje spawneado por piezas
        (CallFunction|PossessCharacter (Utilities|Array|Get(acopy) _outactors 1))
        (Variables|Default|SetUsedCharacter (Utilities|Array|Get(acopy) _outactors 1))
        (Variables|Default|SetCharacterOriginalPosition (Transformation|GetActorLocation (Utilities|Array|Get(acopy) _outactors 1)))
        (if (> (Utilities|Array|Length _outactors) 2)
          (Default|NewMessage (Utilities|Array|Get(acopy) _outactors 1) "Varias piezas de personaje detectadas. Solo se usará la primera.")
          (Utilities|FlowControl|Delay 4.0)
          (Default|DeleteMessage (Utilities|Array|Get(acopy) _outactors 1)))
        (else
          ;;[0.05926 0 0.3647 0.5] Poseer el personaje por defecto de la escena
          (CallFunction|PossessCharacter (Utilities|Array|Get(acopy) _outactors))
          (Variables|Default|SetUsedCharacter (Utilities|Array|Get(acopy) _outactors))
          (Variables|Default|SetCharacterOriginalPosition (Transformation|GetActorLocation (Utilities|Array|Get(acopy) _outactors))))))
    (:B
      (Pawn|UnPossess (Game|GetPlayerController 0))
      (CallFunction|ToggleCMUI)
      (CallFunction|SwitchCamera "CTopdown")
      (Input|SetInputModeUIOnly _returnvalue 0 "DoNotLock" false)
      (Variables|/Script/Engine.PlayerController|SetbShowMouseCursor _returnvalue true)
      (Transformation|SetActorLocation (Variables|Default|GetUsedCharacter) (Variables|Default|GetCharacterOriginalPosition) false false)
      (Transformation|SetActorRotation (Variables|Default|GetUsedCharacter)))))

(event Custom|RotateCTopdownLeft
  (bind _cameras (Variables|Default|GetCameras))
  (bind (_value _returnvalue) (Utilities|Map|Find _cameras "CTopdown"))
  ;[0.1274 0.2159 0.5149 0.502] Rotar suavemente la cámara cenital 90º a izq./der.
  (Variables|Default|SetRotation 9e+01)
  (if (== (Variables|Default|GetCurrentCamera) "CTopdown")
    (Utilities|FlowControl|DoOnce false
      (:Completed
        (if _returnvalue
          (Variables|Default|SetStartCTopdownRotation (Transformation|GetActorRotation _value))
          (bind _rotationoffset (Timeline|CameraRotation PlayFromStart)
            (:Update
              (Transformation|SetActorRotation _value (Math|Rotator|Lerp(Rotator) (Variables|Default|GetStartCTopdownRotation) (Math|Rotator|MakeRotator (+ (.roll (Variables|Default|GetStartCTopdownRotation)) (Variables|Default|GetRotation)) (.pitch (Variables|Default|GetStartCTopdownRotation)) (.yaw (Variables|Default|GetStartCTopdownRotation))) _rotationoffset true)))
            (:Finished
              (CallFunction|FinishedCRotation))))))))

(event Custom|FinishedCRotation
  (bind _cameras (Variables|Default|GetCameras))
  (bind (_value _returnvalue) (Utilities|Map|Find _cameras "CTopdown"))
  ;[0.1274 0.2159 0.5149 0.502] Rotar suavemente la cámara cenital 90º a izq./der.
  (Utilities|FlowControl|DoOnce false) ; enters at Reset
)

(event Custom|SwitchSpectatorCamera
  (bind _currentcamera (Variables|Default|GetCurrentCamera))
  (bind _cameras (Variables|Default|GetCameras))
  (bind (_value _returnvalue) (Utilities|Map|Find _cameras _currentcamera))
  ;[0.1651 0.5029 0.1248 0.502] Cambiar a la cámara libre
  (if _returnvalue
    (Utilities|FlowControl|Sequence
      (:then_0
        (Utilities|FlowControl|DoOnce false
          (:Completed
            (bind _returnvalue_2 (Game|SpawnActorfromClass "/Game/Blueprints/BP_SpectatorCamera.BP_SpectatorCamera_C" (Math|Transform|MakeTransform "0, 0, 0" "0, 0, 0" "1.000000,1.000000,1.000000") "Undefined" "MultiplyWithRoot" 0 0))
            (Variables|Default|SetSpectatorCamera _returnvalue_2)
            (bind _returnvalue_3 (UserInterface|CreateWidget "/Game/UI/WBP_SpectatorCamera.WBP_SpectatorCamera_C"))
            (Variables|Default|SetSpectatorCameraWidget _returnvalue_3)
            (UserInterface|Viewport|AddtoViewport _returnvalue_3 0))))
      (:then_1
        (Transformation|SetActorLocationAndRotation (Variables|Default|GetSpectatorCamera) (Transformation|GetActorLocation _value) (Transformation|GetActorRotation _value))
        (Pawn|Possess (Game|GetPlayerController 0) (Variables|Default|GetSpectatorCamera))
        (CallFunction|ToggleCMUI)
        (Default|DisableBTSpectatorCamera (Variables|Default|GetConstructionWidget))
        (Variables|Default|SetbActiveSpectatorCamera true)
        (Default|DisableBTCTopdownRot (Variables|Default|GetConstructionWidget))))))

(event EventBeginPlay
  (bind _returnvalue (Game|GetPlayerController 0))
  ;[0.15 0.15 0.15 0.5] Al inicio obtener referencias a las cámaras y al UDPReceiver y mostrar la interfaz del modo construcción ocn vista cenital
  (Utilities|FlowControl|Sequence
    (:then_0
      (bind _returnvalue_2 (UserInterface|CreateWidget "/Game/UI/WBP_ConstructionMode.WBP_ConstructionMode_C"))
      (Variables|Default|SetConstructionWidget _returnvalue_2)
      (UserInterface|Viewport|AddtoViewport _returnvalue_2 0)
      (CallFunction|GetCameras)
      (CallFunction|SwitchCamera "CTopdown")
      (Input|SetInputModeUIOnly _returnvalue 0 "DoNotLock" false)
      (Variables|/Script/Engine.PlayerController|SetbShowMouseCursor _returnvalue true))
    (:then_1
      (bind _outactors (Actor|GetAllActorsOfClass "/Game/Blueprints/BP_UDPReceiver.BP_UDPReceiver_C"))
      (Variables|Default|SetUDPReceiver (Utilities|Array|Get(acopy) _outactors)))))

(fn ConstructionScript)