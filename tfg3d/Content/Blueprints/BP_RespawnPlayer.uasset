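; Kill-zone volume that returns a fallen player to their last valid respawn point, with a configurable box extent.
; On overlap by a Player-tagged actor, it plays a sound and fade-out, then after a short delay moves BP_Character above LastValidPlayerRespawnPoint, zeroes its velocity and fades in.
; A parallel Sequence branch resets the DoOnce immediately and removes both fade widgets after a longer delay.
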(event OnComponentBeginOverlap(Collision)
  (params (OverlappedComponent :type Primitive%20Component%20Object%20Reference) (OtherActor :type Actor%20Object%20Reference) (OtherComp :type Primitive%20Component%20Object%20Reference) (OtherBodyIndex :type Integer) (bFromSweep :type Boolean) (SweepResult :type Hit%20Result%20Structure%20%28by%20ref%29))
  ;[0.15 0.15 0.15 0.5] Respawn del jugador en la última posición en la que estuvo antes de caerse del mapa (con FadeIn y FadeOut)
  (if (Actor|ActorHasTag OtherActor "Player")
    (Utilities|FlowControl|DoOnce false
      (:Completed
        (Utilities|FlowControl|Sequence
          (:then_0
            (bind _returnvalue (UserInterface|CreateWidget "/Game/UI/WBP_FadeOut.WBP_FadeOut_C"))
            (Variables|Default|SetFadeOutWidget _returnvalue)
            (UserInterface|Viewport|AddtoViewport _returnvalue 0)
            (Audio|PlaySound2D "/Engine/VREditor/Sounds/UI/Floating_UI_Close.Floating_UI_Close" 1.0 1.0 0.0 0 0)
            (Utilities|FlowControl|Delay 0.5)
            (bind _asbp_character (Utilities|Casting|CastToBP_Character (Game|GetPlayerCharacter 0)))
            (Transformation|SetActorLocation (Game|GetPlayerCharacter 0) (+ (Variables|/Game/Blueprints/BP_Character.BP_Character_C|GetLastValidPlayerRespawnPoint _asbp_character) "0.000000,0.000000,256.000000") false false)
            (Variables|/Script/Engine.MovementComponent|SetVelocity (Variables|/Script/Engine.Character|GetCharacterMovement _asbp_character) "0, 0, 0")
            (bind _returnvalue_2 (UserInterface|CreateWidget "/Game/UI/WBP_FadeIn.WBP_FadeIn_C"))
            (Variables|Default|SetFadeInWidget _returnvalue_2)
            (UserInterface|Viewport|AddtoViewport _returnvalue_2 0))
          (:then_1
            (CallFunction|ResetDoOnce)
            (Utilities|FlowControl|Delay 1.0)
            (Widget|RemovefromParent (Variables|Default|GetFadeInWidget))))))))

(event Custom|ResetDoOnce
  ;[0.15 0.15 0.15 0.5] Respawn del jugador en la última posición en la que estuvo antes de caerse del mapa (con FadeIn y FadeOut)
  (Utilities|FlowControl|DoOnce false) ; enters at Reset
)

(fn ConstructionScript
  ;[0.15 0.15 0.15 0.5] Configurar el tamaño de la colisión
  (Components|Box|SetBoxExtent (Variables|Default|GetCollision) (Variables|Default|GetIn%20Box%20Extent) true))