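; Spike trap Blueprint that raises spikes shortly after a Player-tagged actor enters its collision and damages that actor.
; A timeline lerps the spike mesh up alongside Niagara, sound and light-flicker effects, then starts a delayed loop dealing damage every second while overlap persists.
; Re-entering raised spikes damages immediately.
; A looping timer periodically reverses the timeline to lower them once the stored actor has left.
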(event OnComponentBeginOverlap(Collision)
  (params (OverlappedComponent :type Primitive%20Component%20Object%20Reference) (OtherActor :type Actor%20Object%20Reference) (OtherComp :type Primitive%20Component%20Object%20Reference) (OtherBodyIndex :type Integer) (bFromSweep :type Boolean) (SweepResult :type Hit%20Result%20Structure%20%28by%20ref%29))
  ;[0.149 0.149 0.149 0.502] Si un jugador pisa los pinchos y no estaban subidos, suben tras 0.5 segundos y le hacen daño. Si estaban subidos le daña directamente.
  (if (Actor|ActorHasTag OtherActor "Player")
    (Variables|Default|SetOther%20Actor OtherActor)
    (if (Variables|Default|GetTriggered)
      (CallFunction|DealDamage)
      (else
        (Utilities|Time|SetTimerbyEvent (delegate Custom|ResetSpikeTrap) 4.0 true)
        (Utilities|FlowControl|Delay 0.2)
        (Variables|Default|SetTriggered true)
        (Components|Activation|Activate (Variables|Default|GetNS_Spikes) false)
        (CallFunction|LightFlicker)
        (Audio|Components|Audio|Play (Variables|Default|GetAudioSpikes) 0.0)
        (bind _up (Timeline|T_Spikes Play)
          (:Update
            (Transformation|SetRelativeLocation (Variables|Default|GetSM_Spikes) (Math|Vector|Lerp(Vector) "0.000000,0.000000,-51.000000" "0, 0, 0" _up) false false))
          (:Finished
            (if (Variables|Default|GetTriggered)
              (CallFunction|DealDamage))))))))

(event Custom|ResetSpikeTrap
  ;[0.149 0.149 0.149 0.502] Si un jugador pisa los pinchos y no estaban subidos, suben tras 0.5 segundos y le hacen daño. Si estaban subidos le daña directamente.
  (if (not (Collision|IsOverlappingActor (Variables|Default|GetCollision) (Variables|Default|GetOther%20Actor) :!class /Script/Engine.PrimitiveComponent)) ; Quitar este if y el looping del timer para que tras 4 segundos bajen siempre
    (if (Variables|Default|GetTriggered)
      (Variables|Default|SetTriggered false)
      (Audio|Components|Audio|Play (Variables|Default|GetAudioSpikes) 0.0)
      (bind _up (Timeline|T_Spikes Reverse)
        (:Update
          (Transformation|SetRelativeLocation (Variables|Default|GetSM_Spikes) (Math|Vector|Lerp(Vector) "0.000000,0.000000,-51.000000" "0, 0, 0" _up) false false))
        (:Finished
          (if (Variables|Default|GetTriggered)
            (CallFunction|DealDamage)))))))

(event Custom|DealDamage
  (bind _other_actor (Variables|Default|GetOther%20Actor))
  ;[1 0.4252 0.472 0.5] Si el actor que inició el overlap sique ahí y los pinchos están subidos, le hace daño cada segundo
  (if (and (Collision|IsOverlappingActor (Variables|Default|GetCollision) _other_actor :!class /Script/Engine.PrimitiveComponent) (Variables|Default|GetTriggered)) :!label _label
    (Game|Damage|ApplyDamage _other_actor 0.1 0 0)
    (Utilities|FlowControl|Delay 1.0)
    (goto _label)))

(event Custom|LightFlicker
  ;[0.1248 0.4287 1 0.5] Parpadeo de luz (VFX)
  (for _index (range 0 2)
    (bind _flicker (Timeline|LightFlickerTimeline PlayFromStart)
      (:Update
        (Rendering|Components|Light|SetIntensity (Variables|Default|GetPointLight) (* _flicker 1e+02))))))

(fn ConstructionScript)