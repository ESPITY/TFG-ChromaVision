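; Game mode that runs a construction mode with switchable cameras and hands control to either the player character or a free spectator camera.
; At start it maps CameraActors by tag, opens the top-down view and shows the construction widget.
; Camera switches use blended view targets, while a timeline rotates the top-down camera in guarded 90-degree steps.
; Entering character mode stops the UDP receiver; both possession paths toggle the UI.
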(event Custom|GetCameras
  ;[0.15 0.15 0.15 0.5] Obtener las referencias de las cámaras (value) y guardarlas en un map con el tag (key)
  (bind _outactors (Actor|GetAllActorsOfClass "/Script/Engine.CameraActor"))
  (for _array_element _outactors
    (Utilities|Map|Add (Variables|Default|GetCameras) (Utilities|Array|Get(acopy) (Variables|/Script/Engine.Actor|GetTags _array_element)) _array_element)))

(event Custom|ToggleCMUI
  (bind _returnvalue (Game|GetPlayerController 0))
  (bind _constructionwidget (Variables|Default|GetConstructionWidget))
  ;[0.15 0.15 0.15 0.5] Mostrar/ocultar la interfaz del modo de construcción
  (if (Widget|IsVisible _constructionwidget)
    (Widget|SetVisibility _constructionwidget "Hidden")
    (Input|SetInputModeGameOnly _returnvalue false)
    (Variables|/Script/Engine.PlayerController|SetbShowMouseCursor _returnvalue false)
    (else
      (Widget|SetVisibility _constructionwidget "Visible")
      (Input|SetInputModeGameandUI _returnvalue 0 "DoNotLock" true false)
      (Variables|/Script/Engine.PlayerController|SetbShowMouseCursor _returnvalue true))))

(event Custom|SwitchCamera
  (params (Camera :type Name))
  (bind _returnvalue (Game|GetPlayerController 0))
  (bind _cameras (Variables|Default|GetCameras))
  (bind (_value _returnvalue_2) (Utilities|Map|Find _cameras Camera))
  ;[0.15 0.15 0.15 0.5] Cambiar de cámara con el tag desde el WBP_ConstructionMode
  (if _returnvalue_2
    (Pawn|UnPossess _returnvalue)
    (Utilities|FlowControl|DelayUntilNextTick)
    (Game|Player|SetViewTargetwithBlend _returnvalue _value 0.5 "VTBlend_Cubic" 0.0 false)
    (Variables|Default|SetCurrentCamera Camera)))

(event Custom|RotateCTopdownRight
  (bind _cameras (Variables|Default|GetCameras))
  (bind (_value _returnvalue) (Utilities|Map|Find _cameras "CTopdown"))
  ;[0.15 0.15 0.15 0.5] Rotar suavemente la cámara cenital 90º a izq./der.
  (Variables|Default|SetRotation -9e+01)
  (if (== (Variables|Default|GetCurrentCamera) "CTopdown")
    (Utilities|FlowControl|DoOnce false
      (:Completed
        (if _returnvalue
          (Variables|Default|SetStartCTopdownRotation (Transformation|GetActorRotation _value))
          (bind _rotationoffset (Timeline|CameraRotation PlayFromStart)
            (:Update
              (Transformation|SetActorRotation _value (Math|Rotator|Lerp(Rotator) (Variables|Default|GetStartCTopdownRotation) (Math|Rotator|MakeRotator (+ (.roll (Variables|Default|GetStartCTopdownRotation)) (Variables|Default|GetRotation)) (.pitch (Variables|Default|GetStartCTopdownRotation)) (.yaw (Variables|Default|GetStartCTopdownRotation))) _rotationoffset true)))
            (:Finished
              (CallFunction|FinishedCRotation))))))))

(event Custom|ChangeMode
  (Class|UDPReceiver|StopUDPReceiver (Variables|Default|GetUDPReceiver))
  (bind _outactors (Actor|GetAllActorsOfClasswithTag "/Game/Blueprints/BP_Character.BP_Character_C" "Player"))
  (Pawn|SpawnDefaultController (Utilities|Array|Get(acopy) _outactors))
  (Pawn|Possess (Game|GetPlayerController 0) (Utilities|Array|Get(acopy) _outactors))
  (Default|InitializeCharacter (Utilities|Array|Get(acopy) _outactors))
  (CallFunction|ToggleCMUI))

(event Custom|RotateCTopdownLeft
  (bind _cameras (Variables|Default|GetCameras))
  (bind (_value _returnvalue) (Utilities|Map|Find _cameras "CTopdown"))
  ;[0.15 0.15 0.15 0.5] Rotar suavemente la cámara cenital 90º a izq./der.
  (Variables|Default|SetRotation 9e+01)
  (if (== (Variables|Default|GetCurrentCamera) "CTopdown")
    (Utilities|FlowControl|DoOnce false
      (:Completed
        (if _returnvalue
          (Variables|Default|SetStartCTopdownRotation (Transformation|GetActorRotation _value))
          (bind _rotationoffset (Timeline|CameraRotation PlayFromStart)
            (:Update
              (Transformation|SetActorRotation _value (Math|Rotator|Lerp(Rotator) (Variables|Default|GetStartCTopdownRotation) (Math|Rotator|MakeRotator (+ (.roll (Variables|Default|GetStartCTopdownRotation)) (Variables|Default|GetRotation)) (.pitch (Variables|Default|GetStartCTopdownRotation)) (.yaw (Variables|Default|GetStartCTopdownRotation))) _rotationoffset true)))
            (:Finished
              (CallFunction|FinishedCRotation))))))))

(event Custom|FinishedCRotation
  (bind _cameras (Variables|Default|GetCameras))
  (bind (_value _returnvalue) (Utilities|Map|Find _cameras "CTopdown"))
  ;[0.15 0.15 0.15 0.5] Rotar suavemente la cámara cenital 90º a izq./der.
  (Utilities|FlowControl|DoOnce false) ; enters at Reset
)

(event Custom|SwitchSpectatorCamera
  (bind _currentcamera (Variables|Default|GetCurrentCamera))
  (bind _cameras (Variables|Default|GetCameras))
  (bind (_value _returnvalue) (Utilities|Map|Find _cameras _currentcamera))
  ;[0.15 0.15 0.15 0.5] Cambiar a la cámara libre
  (if _returnvalue
    (Utilities|FlowControl|Sequence
      (:then_0
        (Utilities|FlowControl|DoOnce false
          (:Completed
            (bind _returnvalue_2 (Game|SpawnActorfromClass "/Game/Blueprints/BP_SpectatorCamera.BP_SpectatorCamera_C" (Math|Transform|MakeTransform "0, 0, 0" "0, 0, 0" "1.000000,1.000000,1.000000") "Undefined" "MultiplyWithRoot" 0 0))
            (Variables|Default|SetSpectatorCamera _returnvalue_2))))
      (:then_1
        (Transformation|SetActorLocationAndRotation (Variables|Default|GetSpectatorCamera) (Transformation|GetActorLocation _value) (Transformation|GetActorRotation _value))
        (Pawn|Possess (Game|GetPlayerController 0) (Variables|Default|GetSpectatorCamera))
        (Default|InitializeSpectatorC (Variables|Default|GetSpectatorCamera))
        (CallFunction|ToggleCMUI)))))

(event EventBeginPlay
  (bind _returnvalue (Game|GetPlayerController 0))
  ;[0.15 0.15 0.15 0.5] Comment
  (Utilities|FlowControl|Sequence
    (:then_0
      (CallFunction|GetCameras)
      (CallFunction|SwitchCamera "CTopdown")
      (bind _returnvalue_2 (UserInterface|CreateWidget "/Game/UI/WBP_ConstructionMode.WBP_ConstructionMode_C"))
      (Variables|Default|SetConstructionWidget _returnvalue_2)
      (UserInterface|Viewport|AddtoViewport _returnvalue_2 0)
      (Input|SetInputModeUIOnly _returnvalue 0 "DoNotLock" false)
      (Variables|/Script/Engine.PlayerController|SetbShowMouseCursor _returnvalue true))
    (:then_1
      (bind _outactors (Actor|GetAllActorsOfClass "/Game/Blueprints/BP_UDPReceiver.BP_UDPReceiver_C"))
      (Variables|Default|SetUDPReceiver (Utilities|Array|Get(acopy) _outactors)))))

(fn ConstructionScript)